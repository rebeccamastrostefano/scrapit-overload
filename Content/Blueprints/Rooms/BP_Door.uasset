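; BP_Door is a room door that opens and closes through two events, Open and Close.
; Each event toggles the CollisionSphere, plays an animation on the door skeletal mesh, then after a short delay switches the DoorBlock collision.
; Open enables sphere queries and clears the block, while Close does the reverse.
; The animation names are inverted: Open plays AS_Door_Close and Close plays AS_Door_Open.
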(event EventOpen
  (Collision|SetCollisionEnabled (Variables|Default|GetCollisionSphere) "QueryOnly")
  (Components|Animation|PlayAnimation (Variables|Default|GetSKM_Door) "/Game/Models/Door/AS_Door_Close.AS_Door_Close" false)
  (Utilities|FlowControl|Delay 0.5)
  (Collision|SetCollisionEnabled (Variables|Default|GetDoorBlock) "NoCollision"))

(event EventClose
  (Collision|SetCollisionEnabled (Variables|Default|GetCollisionSphere) "NoCollision")
  (Components|Animation|PlayAnimation (Variables|Default|GetSKM_Door) "/Game/Models/Door/AS_Door_Open.AS_Door_Open" false)
  (Utilities|FlowControl|Delay 0.5)
  (Collision|SetCollisionEnabled (Variables|Default|GetDoorBlock) "PhysicsOnly"))

(fn ConstructionScript)