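; BP_Exit is a room exit trigger that moves the player onward through the run when their pawn overlaps its box.
; It compares the length of the LevelsManager run map with the PersistentManager level rank, opening the Workshop level when they match.
; Otherwise it pauses the game, switches to UI-only input with a visible cursor, and shows a WBP_LevelChoice widget after building its map UI.
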(event OnComponentBeginOverlap(Box)
  (params (OverlappedComponent :type Primitive%20Component%20Object%20Reference) (OtherActor :type Actor%20Object%20Reference) (OtherComp :type Primitive%20Component%20Object%20Reference) (OtherBodyIndex :type Integer) (bFromSweep :type Boolean) (SweepResult :type Hit%20Result%20Structure%20%28by%20ref%29))
  (bind _returnvalue (Game|GetPlayerController 0))
  (if (== OtherActor (Game|Player|GetPlayerPawn 0))
    (bind _returnvalue_2 (Class|LevelsManager|GetRunMap (Subsystems|GetLevelsManager)))
    (if (== (Utilities|Array|Length _returnvalue_2) (Class|PersistentManager|GetLevelRank (Subsystems|GetPersistentManager)))
      (Game|OpenLevel(byObjectReference) "/Game/Levels/Workshop.Workshop")
      (else
        (bind _returnvalue_3 (UserInterface|CreateWidget "/Game/Blueprints/Widgets/LevelsTree/WBP_LevelChoice.WBP_LevelChoice_C" (Game|GetPlayerController 0)))
        (Game|SetGamePaused true)
        (Variables|/Script/Engine.PlayerController|SetbShowMouseCursor _returnvalue true)
        (Input|SetInputModeUIOnly _returnvalue 0 "DoNotLock" false)
        (Default|BuildMapUI _returnvalue_3)
        (UserInterface|Viewport|AddtoViewport _returnvalue_3 0)))))

(fn ConstructionScript)