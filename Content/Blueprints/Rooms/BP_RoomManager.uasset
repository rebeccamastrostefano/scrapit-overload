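; BP_RoomManager runs per-room setup, picking the music for the room and reacting to enemy deaths.
; On BeginPlay it binds to the EnemySpawner's enemy-eliminated event and asks the game instance to crossfade music chosen by room type.
; Special rooms take their track from the LevelsManager's level type, such as shop, treasure or boss.
; Each enemy death plays 2D hit and scrap-burst sounds.
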(event Custom|OnEnemyDeath
  (params (DeathLocation :type Vector) (BaseDropAmount :type Integer))
  (Audio|SpawnSound2D "/Game/Sound/Enemies/SC_HitEnemy.SC_HitEnemy" 1.0 1.0 0.0 0)
  (Audio|SpawnSound2D "/Game/Sound/Enemies/SC_ScrapBurst.SC_ScrapBurst" 1.0 1.0 0.0 0))

(event EventBeginPlay
  (Utilities|FlowControl|Sequence
    (:then_0
      (EventDispatchers|BindEventtoOnEnemyEliminated (Variables|Default|GetEnemySpawner) (delegate Custom|OnEnemyDeath)))
    (:then_1
      ;[0.15 0.15 0.15 0.5] Music
      (bind _asbp_game_instance (Utilities|Casting|CastToBP_GameInstance (Game|GetGameInstance)))
      (Default|CrossFadeMusic _asbp_game_instance (Utilities|Select :Index (Variables|Default|GetRoomType) :Start "/Game/Sound/Music/SW_Start.SW_Start" :Combat "/Game/Sound/Music/SW_Combat.SW_Combat" :Special (Utilities|Select :Index (Class|LevelsManager|GetLevelType (Subsystems|GetLevelsManager)) :Standard "/Game/Sound/Music/SW_Start.SW_Start" :Shop "/Game/Sound/Music/SW_Shop.SW_Shop" :Maintenance "/Game/Sound/Music/SW_Maintenance.SW_Maintenance" :Treasure "/Game/Sound/Music/SW_Treasure.SW_Treasure" :MiniBoss "/Game/Sound/Music/SW_Combat.SW_Combat" :FinalBoss "/Game/Sound/Music/SW_Combat.SW_Combat") :Exit "/Game/Sound/Music/SW_Start.SW_Start")))))

(fn ConstructionScript)