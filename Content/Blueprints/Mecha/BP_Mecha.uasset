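; BP_Mecha is the player's mecha, handling its visual and feedback reactions to magnet, damage, scrap and tier events.
; Tick eases a look-at target toward the nearest enemy and scales smoke Niagara speed with velocity.
; Bound events drive lid and character AnimBPs, feedback, magnet field and scrap burst effects, plus extra smoke at tier five.
; Timelines animate blink and hurt morph targets and mesh scale loop and bounce.
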(event Custom|OnMagnetStateChanged
  (params (bIsActive :type Boolean))
  ;[0.1469 0.09456 0.15 0.5] Feeedbacks
  ;;[0.15 0.15 0.15 0.5] Magnet
  (Utilities|FlowControl|Sequence
    (:then_0
      (bind _asabp_character (Utilities|Casting|CastToABP_Character (Components|SkeletalMesh|GetAnimInstance (Variables|Default|GetSKM_Character))))
      (Variables|/Game/Blueprints/Mecha/ABP_Character.ABP_Character_C|SetOpen _asabp_character bIsActive))
    (:then_1
      (bind _asabp_lid (Utilities|Casting|CastToABP_Lid (Components|SkeletalMesh|GetAnimInstance (Variables|Default|GetSKM_Lid))))
      (Variables|/Game/Blueprints/Mecha/ABP_Lid.ABP_Lid_C|SetOpen _asabp_lid bIsActive))
    (:then_2
      (Default|PlayMagnetFeedback (Variables|Default|GetBP_Feedback) bIsActive)
      (Components|Activation|SetActive (Variables|Default|GetNS_MagnetField) bIsActive false))))

(event Custom|OnBlink
  ;[0.1469 0.09456 0.15 0.5] Feeedbacks
  ;;[0.15 0.15 0.15 0.5] Blink
  (bind _blink (Timeline|Blink PlayFromStart)
    (:Update
      (Components|SkeletalMesh|SetMorphTarget (Variables|Default|GetSKM_Character) "Blink" _blink true))))

(event Custom|ScrapAcquired
  (params (NewScrapCount :type Integer) (bIsIncremental :type Boolean))
  ;[0.1469 0.09456 0.15 0.5] Feeedbacks
  ;;[0.15 0.15 0.15 0.5] Scraps Acquired
  (if (and bIsIncremental (not (Variables|Default|GetIsScaleAnimPlaying)))
    (Variables|Default|SetIsScaleAnimPlaying true)
    (bind _scale (Timeline|ScaleBounce PlayFromStart)
      (:Update
        (Transformation|SetRelativeScale3D (Variables|Default|GetMechaMesh) _scale))
      (:Finished
        (Variables|Default|SetIsScaleAnimPlaying false)))))

(event Custom|OnHurt
  (params (bOnShield :type Boolean))
  (bind _returnvalue (Transformation|GetActorLocation))
  (bind (_x _y _z) (Math|Vector|BreakVector _returnvalue))
  ;[0.1469 0.09456 0.15 0.5] Feeedbacks
  ;;[0.15 0.15 0.15 0.5] Take Damage
  (Utilities|FlowControl|Sequence
    (:then_0
      (Default|PlayHurtFeedback (Variables|Default|GetBP_Feedback))
      (bind _blink (Timeline|Timeline PlayFromStart)
        (:Update
          (Components|SkeletalMesh|SetMorphTarget (Variables|Default|GetSKM_Character) "Hurt" _blink true))))
    (:then_1
      (if bOnShield
        (Niagara|SpawnSystematLocation (Variables|Default|GetScrapBurstNiagara) (Math|Vector|MakeVector _x _y (+ _z 1e+02)) "0, 0, 0" "1.000000,1.000000,1.000000" true true "AutoRelease")))))

(event Custom|OnTierChanged
  (params (Tier :type Mass%20Tier%20Structure))
  ;[0.1469 0.09456 0.15 0.5] Feeedbacks
  (if (== (.tiernumber Tier) 5)
    (Components|Activation|Activate (Variables|Default|GetNS_Smoke2) false)
    (Components|Activation|Activate (Variables|Default|GetNS_Smoke1) false)))

(event EventBeginPlay
  ;[0.1469 0.09456 0.15 0.5] Feeedbacks
  (Utilities|FlowControl|Sequence
    (:then_0
      ;;[0.15 0.15 0.15 0.5] Magnet
      (EventDispatchers|BindEventtoOnMagnetStateChange (delegate Custom|OnMagnetStateChanged)))
    (:then_1
      ;;[0.15 0.15 0.15 0.5] Blink
      (Utilities|Time|SetTimerbyEvent (delegate Custom|OnBlink) 5.0 true))
    (:then_2
      ;;[0.15 0.15 0.15 0.5] Take Damage
      (EventDispatchers|BindEventtoOnPlayerTakeDamage (delegate Custom|OnHurt)))
    (:then_3
      ;;[0.15 0.15 0.15 0.5] Scraps Acquired
      (EventDispatchers|BindEventtoOnScrapCountChanged (delegate Custom|ScrapAcquired)))
    (:then_4
      (EventDispatchers|BindEventtoOnTierChanged (Variables|Default|GetTierSystem) (delegate Custom|OnTierChanged)))
    (:then_5
      (bind _scalevec (Timeline|ScaleLoop Play)
        (:Update
          (Transformation|SetRelativeScale3D (Variables|Default|GetMechaMesh) _scalevec))))))

(event EventTick
  (params (DeltaSeconds :type Float%20%28single-precision%29))
  (bind _returnvalue (Transformation|GetVelocity))
  (bind _returnvalue_2 (Math|Vector|VectorLength _returnvalue))
  (bind _returnvalue_3 (/ _returnvalue_2 2e+01))
  (bind _returnvalue_4 (+ _returnvalue_3 5.0))
  ;[0.15 0.09492 0.0565 0.5] Look At Target Update
  (Utilities|FlowControl|Sequence
    (:then_0
      (bind _returnvalue_5 (Class|FunctionLibrary|GetClosestEnemy self 5e+02))
      (if (Utilities|IsValid _returnvalue_5)
        (bind _output_get (Variables|Default|SetNearestEnemy _returnvalue_5))
        (Variables|Default|SetSmoothLookAtTarget (Math|Interpolation|VInterpTo (Variables|Default|GetSmoothLookAtTarget) (Math|Vector|MakeVector (.X (Math|Vector|BreakVector (Transformation|GetActorLocation _output_get))) (.Y (Math|Vector|BreakVector (Transformation|GetActorLocation _output_get))) 1.5e+02) DeltaSeconds 5.0))))
    (:then_1
      ;[0.15 0.15 0.15 0.5] Smoke VFx
      (Niagara|SetNiagaraVariable(Float) (Variables|Default|GetNS_Smoke) "speed" _returnvalue_4)
      (Niagara|SetNiagaraVariable(Float) (Variables|Default|GetNS_Smoke2) "speed" _returnvalue_4)
      (Niagara|SetNiagaraVariable(Float) (Variables|Default|GetNS_Smoke1) "speed" _returnvalue_4))))

(fn ConstructionScript)