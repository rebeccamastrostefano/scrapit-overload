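; BP_Feedback is a blueprint that plays player feedback effects for getting hurt and for a magnet state.
; On BeginPlay it creates a level sequence player from the hurt sequence and keeps it for reuse.
; Hurt feedback plays that sequence and starts a hurt camera shake on the first player controller.
; Magnet feedback starts or immediately stops its own camera shake depending on an active flag.
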(event Custom|PlayHurtFeedback
  (Sequencer|Player|Play (Variables|Default|GetPlayer_Hurt) :!class /Script/MovieScene.MovieSceneSequencePlayer)
  (Game|Feedback|ClientStartCameraShake (Game|GetPlayerController 0) (Variables|Default|GetCameraShakerHurt) 1.0 "CameraLocal" "0, 0, 0"))

(event Custom|PlayMagnetFeedback
  (params (IsActive :type Boolean))
  (bind _returnvalue (Game|GetPlayerController 0))
  (bind _camerashakermagnet (Variables|Default|GetCameraShakerMagnet))
  (if IsActive
    (Game|Feedback|ClientStartCameraShake _returnvalue _camerashakermagnet 1.0 "CameraLocal" "0, 0, 0")
    (else
      (Game|Feedback|ClientStopCameraShake _returnvalue _camerashakermagnet true))))

(event EventBeginPlay
  (bind _returnvalue (Sequencer|Player|CreateLevelSequencePlayer (Variables|Default|GetHurtSequence)))
  (Variables|Default|SetPlayer_Hurt _returnvalue))